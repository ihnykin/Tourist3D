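; Actor component that deals damage of a configured DamageType to one target actor, either once or periodically.
; StartApplyDamage stops any previous target, applies damage immediately, then starts a looping timer if the damage period is positive.
; Damage and period come from the DT_DamageInfo row named after the enum value, with an error logged when missing.
; StopApplyDamage clears the target and timer.
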(event Custom|StartApplyDamage
  (params (Actor :type Actor%20Object%20Reference))
  (Utilities|FlowControl|Sequence
    (:then_0
      (CallFunction|StopApplyDamage))
    (:then_1
      (Variables|Default|SetDamagedActorPrivate Actor)
      (CallFunction|ApplyDamagePrivate))
    (:then_2
      (bind _row (CallFunction|GetDamageInfoPrivate))
      (if (> (.period _row) 0.0)
        (bind _returnvalue (Utilities|Time|SetTimerbyEvent (EventDispatchers|CreateEvent :!event ApplyDamagePrivate) (.period _row) true))
        (Variables|Default|SetDamagedTimerPrivate _returnvalue)))))

(event Custom|StopApplyDamage
  (Variables|Default|SetDamagedActorPrivate 0)
  (Utilities|Time|ClearandInvalidateTimerbyHandle (Variables|Default|GetDamagedTimerPrivate)))

(fn GetDamageInfoPrivate
  (bind _damagetype (Variables|Custom|GetDamageType))
  (bind _returnvalue (Utilities|String|EnumtoString _damagetype))
  (bind _returnvalue_2 (Utilities|GetDataTableRow "/Game/Tourist3D/Blueprints/Components/DamageComponent/DT_DamageInfo.DT_DamageInfo" (Utilities|String|StringToName _returnvalue))
    (:then
      (return _returnvalue_2))
    (:RowNotFound
      (CallFunction|DebugError (Components|GetOwner) "no damage found for: " _returnvalue)
      (return ""))))

(fn ApplyDamagePrivate
  (bind _row (CallFunction|GetDamageInfoPrivate))
  (Game|Damage|ApplyDamage (Variables|Default|GetDamagedActorPrivate) (.damage _row) 0 0))