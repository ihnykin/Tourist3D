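; BP_DamagePawnPlane is an environment plane that damages overlapping actors and tints the screen while the camera is beneath it.
; Begin and end overlap start and stop damage through BPCDamageComponent.
; Tick tests the player camera position against the static mesh plane, skipping a zero location, then fades the screen to UnderPlaneColor or unfades it.
; A flag ensures each fade triggers only when the camera crosses the plane.
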(event Collision|EventActorEndOverlap
  (params (OtherActor :type Actor%20Object%20Reference))
  (Default|StopApplyDamage (Variables|Custom|GetBPC_DamageComponent)))

(event Collision|EventActorBeginOverlap
  (params (OtherActor :type Actor%20Object%20Reference))
  (Default|StartApplyDamage (Variables|Custom|GetBPC_DamageComponent) OtherActor))

(event EventTick
  (params (DeltaSeconds :type Float%20%28single-precision%29))
  (bind _effectprovider (CallFunction|GetMyEffectProvider))
  (bind _returnvalue (Game|GetPlayerCameraManager 0))
  (bind _effect (Default|GetScreenFadeEffect _effectprovider))
  (bind _transformcomponent (Variables|/Script/Engine.PlayerCameraManager|GetTransformComponent _returnvalue))
  (bind _returnvalue_2 (Transformation|GetWorldLocation _transformcomponent))
  (if (Class|KismetMathLibrary|NotEqualExactlyVectorVector _returnvalue_2 "0, 0, 0")
    (bind _isunder (CallFunction|IsPointUnderPlane (Variables|Debug|GetStaticMeshComponent) _returnvalue_2 -0.0016))
    (if _isunder
      (if (not (Variables|Default|GetIsCameraFadingPrivate))
        (Default|StartFade _effect (Variables|Custom|GetUnderPlaneColor) 0.2 false)
        (Variables|Default|SetIsCameraFadingPrivate true))
      (elif (Variables|Default|GetIsCameraFadingPrivate)
        (Default|StartUnfade _effect true)
        (Variables|Default|SetIsCameraFadingPrivate false)))))

(fn ConstructionScript)