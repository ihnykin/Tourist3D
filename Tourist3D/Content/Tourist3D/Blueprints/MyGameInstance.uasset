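; Game instance for Tourist3D that creates the effect provider and logs level load and unload events.
; On Init it spawns a BP_EffectProvider actor at the world origin, always spawning regardless of collision, and stores it in EffectProvider.
; The LoadLevel and UnloadLevel events only write the level name to DebugInfo, and the unload Reason is unused.
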(event Custom|Event%20LoadLevel
  (params (LevelName :type String))
  (CallFunction|DebugInfo self "Load level: " LevelName))

(event Custom|Event%20UnloadLevel
  (params (LevelName :type String) (Reason :type EEndPlayReason%20Enum :default "Destroyed"))
  (CallFunction|DebugInfo self "Unload level: " LevelName))

(event EventInit
  (bind _returnvalue (Game|SpawnActorfromClass "/Game/Tourist3D/Blueprints/Effects/BP_EffectProvider.BP_EffectProvider_C" (Math|Transform|MakeTransform "0, 0, 0") "AlwaysSpawn" 0 0))
  (Variables|Default|SetEffectProvider _returnvalue)
  (CallFunction|DebugInfo self "Init effect provider"))