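; Player character for Tourist3D that handles movement, health and boarding a space rocket.
; Axis input drives yaw-relative forward movement, turning and looking, with jump on action or touch and no strafing.
; Game settings scale frame-time-based rotation and set walk speed, which refreshes when settings are saved.
; While alive, damage lowers health and fires health-changed and death notifications, and overlapping BP_SpaceRocket fires a player-in-rocket notification.
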(event Custom|OnGameSettingsUpdated_CustomEvent
  ;[1 1 0] Update controls if game settings changed
  (Variables|/Script/Engine.CharacterMovementComponent|SetMaxWalkSpeed (Variables|Character|GetCharacterMovement) (* (Variables|/Game/Tourist3D/Blueprints/Core/Providers/SaveGameProvider/BP_SaveGameProvider.BP_SaveGameProvider_C|GetWalkSpeed (CallFunction|GetMyGameSettings)) 1e+02)))

(event EventBeginPlay
  ;[1 1 0] Update controls if game settings changed
  (EventDispatchers|BindEventtoOnGameSettingsSaved (CallFunction|GetMyGameInstance) (delegate Custom|OnGameSettingsUpdated_CustomEvent))
  (Variables|/Script/Engine.CharacterMovementComponent|SetMaxWalkSpeed (Variables|Character|GetCharacterMovement) (* (Variables|/Game/Tourist3D/Blueprints/Core/Providers/SaveGameProvider/BP_SaveGameProvider.BP_SaveGameProvider_C|GetWalkSpeed (CallFunction|GetMyGameSettings)) 1e+02)))

(event Game|Damage|EventAnyDamage
  (params (Damage :type Float%20%28single-precision%29) (DamageType :type Damage%20Type%20Object%20Reference) (InstigatedBy :type Controller%20Object%20Reference) (DamageCauser :type Actor%20Object%20Reference))
  ;[1 0 1] Actions
  (if (CallFunction|IsNotDead)
    (bind _output_get (Variables|Default|SetHealth (Math|Float|Max(Float) (- (Variables|Default|GetHealth) Damage) 0.0)))
    (Default|CallOnPlayerHealthChanged _output_get)
    (if (<= _output_get 0.0)
      (Default|CallOnPlayerDied))))

(event Collision|EventActorBeginOverlap
  (params (OtherActor :type Actor%20Object%20Reference))
  ;[1 0 1] Actions
  (if (CallFunction|IsNotDead)
    (Utilities|Casting|CastToBP_SpaceRocket OtherActor)
    (Default|CallOnPlayerinRocket)))

(event Input|ActionEvents|InputActionJump
  (params (Key :type Key%20Structure :default "None"))
  ;[1 1 1] Input. Jump
  (:Pressed
    (Character|Jump))
  (:Released
    (Character|StopJumping)))

(event Input|AxisEvents|InputAxisMoveForward
  (params (AxisValue :type Float%20%28single-precision%29))
  ;[1 1 1] Input. Move Forward & Backward
  (Pawn|Input|AddMovementInput (Math|Vector|GetForwardVector (Math|Rotator|MakeRotator 0.0 0.0 (.yaw (Pawn|GetControlRotation :!class /Script/Engine.Pawn)))) AxisValue false))

(event Input|AxisEvents|InputAxisLookUpDown
  (params (AxisValue :type Float%20%28single-precision%29))
  ;[1 1 1] Input. Look Up & Down
  (Pawn|Input|AddControllerPitchInput (* AxisValue (Variables|/Game/Tourist3D/Blueprints/Core/Providers/SaveGameProvider/BP_SaveGameProvider.BP_SaveGameProvider_C|GetLookRotationSpeed (CallFunction|GetMyGameSettings)) 6.0 (Utilities|Time|GetWorldDeltaSeconds))))

(event Input|AxisEvents|InputAxisTurnLeftRight
  (params (AxisValue :type Float%20%28single-precision%29))
  ;[1 1 1] Input. Turn Left & Right
  (Pawn|Input|AddControllerYawInput (* AxisValue (Variables|/Game/Tourist3D/Blueprints/Core/Providers/SaveGameProvider/BP_SaveGameProvider.BP_SaveGameProvider_C|GetMoveRotationSpeed (CallFunction|GetMyGameSettings)) 8.0 (Utilities|Time|GetWorldDeltaSeconds))))

(event Input|TouchEvents|InputTouch
  (params (Location :type Vector) (FingerIndex :type ETouchIndex%20Enum))
  ;[1 1 1] Input. Jump (Touch)
  (:Pressed
    (Character|Jump))
  (:Released
    (Character|StopJumping)))

(fn ConstructionScript)

(fn IsDead
  (return (<= (Variables|Default|GetHealth) 0.0)))

(fn IsNotDead
  (return (not (CallFunction|IsDead))))