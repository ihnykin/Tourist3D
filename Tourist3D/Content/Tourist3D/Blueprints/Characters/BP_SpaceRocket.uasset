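; BP_SpaceRocket is a rocket actor that moves between a takeoff point and a landing point.
; BeginPlay caches its starting location as the takeoff point and adds the LandingPoint offset to it for the landing point.
; The Landing event plays a timeline that lerps the actor's location between the two points without sweeping.
; The Takeoff event reverses that same timeline from the end, returning the rocket to its starting location.
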(event Custom|Takeoff
  (bind _alpha (Timeline|TimelineLanding ReverseFromEnd)
    (:Update
      (Transformation|SetActorLocation (Math|Vector|Lerp(Vector) (Variables|Default|GetTakeoffWorldPoint) (Variables|Default|GetLandingWorldPoint) _alpha) false false))))

(event Custom|Landing
  (bind _alpha (Timeline|TimelineLanding PlayFromStart)
    (:Update
      (Transformation|SetActorLocation (Math|Vector|Lerp(Vector) (Variables|Default|GetTakeoffWorldPoint) (Variables|Default|GetLandingWorldPoint) _alpha) false false))))

(event EventBeginPlay
  (Variables|Default|SetTakeoffWorldPoint (Transformation|GetActorLocation))
  (Variables|Default|SetLandingWorldPoint (+ (Variables|Components|GetLandingPoint) (Transformation|GetActorLocation))))

(fn ConstructionScript)