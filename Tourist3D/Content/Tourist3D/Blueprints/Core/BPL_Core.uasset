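; Blueprint function library for Tourist3D that gives global access to the game's core providers through the custom game instance.
; GetMyGameInstance casts the current game instance to MyGameInstance and reports a debug error if the cast fails.
; The other getters use it to return the save game (as game settings), level, level targets, UI and effect providers.
; The level targets getter also calls Initialize on its provider before returning it.
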(fn GetMyGameInstance
  (bind _asmy_game_instance (Utilities|Casting|CastToMyGameInstance (Game|GetGameInstance (LocalVariables|Get__WorldContext)))
    (:then
      _)
    (:CastFailed
      (Utilities|DebugError 0 "BPL_Common | " "Bad game instance"
        (:Out
          _))))
  (return _asmy_game_instance))

(fn GetMyGameSettings
  (return (Variables|/Game/Tourist3D/Blueprints/Core/MyGameInstance.MyGameInstance_C|GetSaveGameProvider (Core|GetMyGameInstance (LocalVariables|Get__WorldContext)))))

(fn GetMyLevelProvider
  (return (Variables|/Game/Tourist3D/Blueprints/Core/MyGameInstance.MyGameInstance_C|GetLevelProvider (Core|GetMyGameInstance (LocalVariables|Get__WorldContext)))))

(fn GetMyLevelTargetsProvider
  (bind ___worldcontext (LocalVariables|Get__WorldContext))
  (bind _gameinstance (Core|GetMyGameInstance ___worldcontext))
  (bind _leveltargetsprovider (Variables|/Game/Tourist3D/Blueprints/Core/MyGameInstance.MyGameInstance_C|GetLevelTargetsProvider _gameinstance))
  (Default|Initialize _leveltargetsprovider false)
  (return _leveltargetsprovider))

(fn GetMyUIProvider
  (return (Variables|/Game/Tourist3D/Blueprints/Core/MyGameInstance.MyGameInstance_C|GetUIProvider (Core|GetMyGameInstance (LocalVariables|Get__WorldContext)))))

(fn GetMyEffectProvider
  (return (Variables|/Game/Tourist3D/Blueprints/Core/MyGameInstance.MyGameInstance_C|GetEffectProvider (Core|GetMyGameInstance (LocalVariables|Get__WorldContext)))))