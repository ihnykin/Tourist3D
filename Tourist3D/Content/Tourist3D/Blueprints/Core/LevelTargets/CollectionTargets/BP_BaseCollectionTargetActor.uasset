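; Base collectible actor for collection level targets, picked up on overlap and reported through an OnCollected event dispatcher.
; On BeginPlay it applies TargetMesh to its static mesh and binds that component's begin overlap.
; Any overlap, with no check on the other actor, broadcasts the target's reference, name and count, plays a click sound at its location and destroys the actor.
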(event Custom|OnCollected_Event
  (params (OverlappedComponent :type Primitive%20Component%20Object%20Reference) (OtherActor :type Actor%20Object%20Reference) (OtherComp :type Primitive%20Component%20Object%20Reference) (OtherBodyIndex :type Integer) (bFromSweep :type Boolean) (SweepResult :type Hit%20Result%20Structure%20%28by%20ref%29))
  (Default|CallOnCollected self (Variables|Custom|GetTargetName) (Variables|Custom|GetTargetCount))
  (Audio|PlaySoundatLocation "/Game/Tourist3D/Resources/Sound/Click/click.Click" (Transformation|GetActorLocation) "0, 0, 0" 1.0 1.0 0.0 0 0 0)
  (Actor|DestroyActor))

(event EventBeginPlay
  (Components|StaticMesh|SetStaticMesh (Variables|Default|GetStaticMesh) (Variables|Custom|GetTargetMesh))
  (Collision|BindEventtoOnComponentBeginOverlap (Variables|Default|GetStaticMesh) (delegate Custom|OnCollected_Event)))

(fn ConstructionScript)