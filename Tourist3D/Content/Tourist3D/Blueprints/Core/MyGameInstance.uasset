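; Game instance for Tourist3D that owns persistent settings and per-level service actors.
; On init it async-loads a save-game provider from a slot, creating a fresh one on failure, and saves it asynchronously when a level unloads.
; On each level load it spawns level, UI and effect providers plus a play-states actor, and finds the placed level targets provider.
; Load and save completion fire notification calls.
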(event Custom|Event%20OnLevelLoaded
  (params (LevelName :type String))
  (Utilities|DebugInfo self "Level loaded: " LevelName
    (:Out
      (CallFunction|InitProviders)
      (CallFunction|InitPlayStates))))

(event Custom|Event%20OnLevelUnloaded
  (params (LevelName :type String) (Reason :type EEndPlayReason%20Enum :default "Destroyed"))
  (Utilities|DebugInfo self "Level unloaded: " LevelName
    (:Out
      (CallFunction|SaveGameSettings))))

(event Custom|SaveGameSettings
  (bind _self self)
  ;[1 1 1] Load/Save game settings
  (bind _bsuccess (|AsyncSaveGametoSlot (Variables|SaveGame|GetSaveGameProvider) (Variables|SaveGame|GetSaveGameSlot) (Variables|SaveGame|GetSaveUserIndex))
    (:Completed
      (if _bsuccess
        (Utilities|DebugInfo _self "SaveGameSettings OK"
          (:Out
            (Default|CallOnGameSettingsSaved)))
        (else
          (Utilities|DebugError _self "SaveGameSettings FAILED"))))))

(event Custom|LoadGameSettings
  ;[1 1 1] Load/Save game settings
  (bind (_savegame _bsuccess) (|AsyncLoadGamefromSlot (Variables|SaveGame|GetSaveGameSlot) (Variables|SaveGame|GetSaveUserIndex))
    (:Completed
      (if _bsuccess
        (bind _asbp_save_game_provider (Utilities|Casting|CastToBP_SaveGameProvider _savegame)
          (:then
            (Variables|SaveGame|SetSaveGameProvider _asbp_save_game_provider))
          (:CastFailed
            (bind _returnvalue (SaveGame|CreateSaveGameObject "/Game/Tourist3D/Blueprints/Core/Providers/SaveGameProvider/BP_SaveGameProvider.BP_SaveGameProvider_C" :!label _label))
            (Variables|SaveGame|SetSaveGameProvider _returnvalue)))
        (else
          (goto _label)))
      (Utilities|DebugInfo self "LoadGameSettings OK"
        (:Out
          (Default|CallOnGameSettingsLoaded))))))

(event EventInit
  (Utilities|DebugInfo self "Init GameInstance"
    (:Out
      (CallFunction|LoadGameSettings))))

(fn InitProviders
  (bind _returnvalue (Math|Transform|MakeTransform "0, 0, 0"))
  (Utilities|FlowControl|Sequence
    (:then_0
      (bind _returnvalue_2 (Game|SpawnActorfromClass "/Game/Tourist3D/Blueprints/Core/Providers/LevelProvider/BP_LevelProvider.BP_LevelProvider_C" _returnvalue "AlwaysSpawn" 0 0))
      (Variables|Default|SetLevelProvider _returnvalue_2)
      (Utilities|DebugInfo self "Init LevelProvider"))
    (:then_1
      (bind _returnvalue_3 (Actor|GetActorOfClass "/Game/Tourist3D/Blueprints/Core/Providers/LevelTargetsProvider/BP_LevelTargetsProvider.BP_LevelTargetsProvider_C"))
      (bind _output_get (Variables|Default|SetLevelTargetsProvider _returnvalue_3))
      (Utilities|DebugInfo self "Init LevelTargetsProvider: " (Utilities|String|ToString(Boolean) (Utilities|IsValid _output_get))))
    (:then_2
      (bind _returnvalue_4 (Game|SpawnActorfromClass "/Game/Tourist3D/UI/BP_UIProvider.BP_UIProvider_C" _returnvalue "AlwaysSpawn" 0 0))
      (Variables|Default|SetUIProvider _returnvalue_4)
      (Utilities|DebugInfo self "Init UIProvider"))
    (:then_3
      (bind _returnvalue_5 (Game|SpawnActorfromClass "/Game/Tourist3D/Blueprints/Core/Providers/EffectsProvider/BP_EffectProvider.BP_EffectProvider_C" _returnvalue "AlwaysSpawn" 0 0))
      (Variables|Default|SetEffectProvider _returnvalue_5)
      (Utilities|DebugInfo self "Init EffectProvider"))))

(fn InitPlayStates
  (bind _returnvalue (Game|SpawnActorfromClass "/Game/Tourist3D/Blueprints/Core/MyLevelPlayStates.MyLevelPlayStates_C" (Math|Transform|MakeTransform "0, 0, 0") "AlwaysSpawn" 0 0))
  (Variables|Default|SetLevelPlayStates _returnvalue)
  (Utilities|DebugInfo self "Init LevelPlayStates"))