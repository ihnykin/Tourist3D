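; Level play-state actor that stages the player's arrival by rocket in Tourist3D.
; On BeginPlay, any level not flagged as the start level plays the landing: space fades away while the BP_SpaceRocket found on the map lands.
; When the flight finishes, the screen fades to black, the controller possesses the placed BP_PlayerCharacter, the HUD opens and the view unfades.
; Missing actors log debug errors; PlayRocketTakeoff is an empty stub, with takeoff nodes left disconnected.
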(event Custom|PlayStartLevel
  ;[1 1 1] Start Level State
  (bind _isstartlevel (Default|IsStartLevel (CallFunction|GetMyLevelProvider)))
  (if (not _isstartlevel)
    (CallFunction|PlayRocketLanding)))

(event Custom|PlayRocketTakeoff)

(event Custom|CustomEvent_OnRocketLandingFinished
  (bind _effectprovider (CallFunction|GetMyEffectProvider))
  (bind _effect (Default|GetScreenFadeEffect _effectprovider))
  ;[1 1 1] Rocket Landing State: land rocket from cosmos with effects and transfer control to the player
  (Default|StartFade _effect "(R=0.000000,G=0.000000,B=0.000000,A=1.000000)" 1.0 false)
  (Utilities|FlowControl|Delay 1.0)
  (bind _playercharacter (CallFunction|FindPlayerCharacter))
  (Pawn|Possess (Game|GetPlayerController 0) _playercharacter)
  (Default|OpenHUD (CallFunction|GetMyUIProvider))
  (Default|StartUnfade _effect true))

(event Custom|PlayRocketLanding
  ;[1 1 1] Rocket Landing State: land rocket from cosmos with effects and transfer control to the player
  (Utilities|FlowControl|Sequence
    (:then_0
      (Default|HideSpace (Default|GetSpaceFadeEffect (CallFunction|GetMyEffectProvider)) 2.0 true))
    (:then_1
      (bind _spacerocket (CallFunction|FindSpaceRocket))
      (Default|RocketLanding _spacerocket)
      (EventDispatchers|BindEventtoOnFlightFinished _spacerocket (delegate Custom|CustomEvent_OnRocketLandingFinished)))))

(event EventBeginPlay
  (CallFunction|PlayStartLevel))

(fn ConstructionScript)

(fn FindSpaceRocket
  (bind _returnvalue (Actor|GetActorOfClass "/Game/Tourist3D/Blueprints/Characters/BP_SpaceRocket.BP_SpaceRocket_C"))
  (Utilities|IsValid _returnvalue
    (:Is%20Valid
      (return _returnvalue))
    (:Is%20Not%20Valid
      (Utilities|DebugError self "No space rocket found. Add BP_SpaceRocket on map."))))

(fn FindPlayerCharacter
  (bind _returnvalue (Actor|GetActorOfClass "/Game/Tourist3D/Blueprints/Characters/BP_PlayerCharacter.BP_PlayerCharacter_C"))
  (Utilities|IsValid _returnvalue
    (:Is%20Valid
      (return _returnvalue))
    (:Is%20Not%20Valid
      (Utilities|DebugError self "No player character found. Add BP_PlayerCharacter on map."))))