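; Level-wide tracker of collection targets, keeping initial and collected amounts for each target name.
; On BeginPlay it finds all BP_BaseCollectionTarget actors, binds to their collected events and counts them per name in an IntVector map (X initial, Y collected).
; Each collection adds the target's weight to Y, rebroadcasts the event and prints totals in debug builds.
; A getter exposes both amounts by name.
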(event Custom|OnCollectionTargetCollected_CustomEvent
  (params (TargetActor :type BP%20Base%20Collection%20Target%20Object%20Reference) (TargetName :type ETargetName%20Enum :default "NewEnumerator2") (TargetWeight :type Integer))
  (CollectionTargets|AddCollectionTarget TargetName TargetWeight)
  (Default|CallOnCollectionTargetCollected TargetName TargetWeight)
  (CollectionTargets|PrintCollectionTargets))

(event EventBeginPlay
  (CollectionTargets|InitCollectionTargets))

(fn ConstructionScript)

(fn InitCollectionTargets
  (bind _collectiontargets (Variables|Default|GetCollectionTargets))
  (bind _outactors (Actor|GetAllActorsOfClass "/Game/Tourist3D/Blueprints/Core/LevelTargetsProvider/CollectionTargets/BP_BaseCollectionTarget.BP_BaseCollectionTarget_C"))
  (for _array_element _outactors
    (EventDispatchers|BindEventtoOnTargetCollected _array_element (EventDispatchers|CreateEvent :!event Custom|OnCollectionTargetCollected_CustomEvent))
    ;[1 1 1] [CollectionTargets]
    ; (TargetName) -> (X = InitialTargetsAmount, Y = CollectedTargetsAmount, Z = 0)
    (if (.ReturnValue (Utilities|Map|Find (Variables|Default|GetCollectionTargets) (Variables|/Game/Tourist3D/Blueprints/Core/LevelTargetsProvider/CollectionTargets/BP_BaseCollectionTarget.BP_BaseCollectionTarget_C|GetTargetName _array_element)))
      (Utilities|Map|Add _collectiontargets (Variables|/Game/Tourist3D/Blueprints/Core/LevelTargetsProvider/CollectionTargets/BP_BaseCollectionTarget.BP_BaseCollectionTarget_C|GetTargetName _array_element) (Utilities|Struct|MakeIntVector (+ (.x (.Value (Utilities|Map|Find (Variables|Default|GetCollectionTargets) (Variables|/Game/Tourist3D/Blueprints/Core/LevelTargetsProvider/CollectionTargets/BP_BaseCollectionTarget.BP_BaseCollectionTarget_C|GetTargetName _array_element)))) 1) 0))
      (else
        (Utilities|Map|Add _collectiontargets (Variables|/Game/Tourist3D/Blueprints/Core/LevelTargetsProvider/CollectionTargets/BP_BaseCollectionTarget.BP_BaseCollectionTarget_C|GetTargetName _array_element) (Utilities|Struct|MakeIntVector 1 0))))))

(fn AddCollectionTarget
  (params (TargetName :type ETargetName%20Enum :default "NewEnumerator2") (TargetWeight :type Integer))
  (bind _collectiontargets (Variables|Default|GetCollectionTargets))
  (bind _value (Utilities|Map|Find _collectiontargets TargetName))
  ;[1 1 1] [CollectionTargets]
  ; (TargetName) -> (X = InitialTargetsAmount, Y = CollectedTargetsAmount, Z = 0)
  (Utilities|Map|Add (Variables|Default|GetCollectionTargets) TargetName (Utilities|Struct|MakeIntVector (.x _value) (+ TargetWeight (.y _value)) (.z _value))))

(fn GetCollectionTarget
  (params (TargetName :type ETargetName%20Enum :default "NewEnumerator2"))
  (bind _collectiontargets (Variables|Default|GetCollectionTargets))
  (bind _value (Utilities|Map|Find _collectiontargets TargetName))
  ;[1 1 1] [CollectionTargets]
  ; (TargetName) -> (X = InitialTargetsAmount, Y = CollectedTargetsAmount, Z = 0)
  (return (.x _value) (.y _value)))

(fn PrintCollectionTargets
  (bind _collectiontargets (Variables|Default|GetCollectionTargets))
  (if (Class|CommonUtils|IsDebugBuild)
    (bind _keys (Utilities|Map|Keys _collectiontargets))
    (for _array_element _keys
      (Utilities|DebugInfo self (Utilities|String|EnumtoString _array_element) (Utilities|String|Append " | Data: " (Utilities|String|ToString(Integer) (.Value (Utilities|Map|Find _collectiontargets _array_element))))))))