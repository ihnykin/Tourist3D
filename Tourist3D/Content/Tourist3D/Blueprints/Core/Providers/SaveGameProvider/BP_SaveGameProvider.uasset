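; BP_SaveGameProvider holds the player's progress stats: gold and the list of completed level names.
; It exposes functions to adjust gold without going negative, record completed maps uniquely, and check whether a map is completed.
; GetStats raises stored gold to a minimum as a bankruptcy guard, so reading stats can change state.
; GetStatsString builds a text summary through GetStats, so it triggers the same guard.
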(fn GetStats
  ;[1 1 1] Prevent bankruptcy
  (Variables|Default|SetGold (Math|Integer|Max(Integer) (Variables|Default|GetGold) 99))
  (return (Variables|Default|GetGold) (Variables|Default|GetCompletedLevels)))

(fn GetStatsString
  (bind (_gold _completedlevels) (CallFunction|GetStats))
  (return (Utilities|String|Append "Gold: " (Utilities|String|ToString(Integer) _gold) " CompletedLevels: " (Class|CommonUtils|NameArraytoString _completedlevels false))))

(fn AddGold
  (params (Add :type Integer))
  (bind _output_get (Variables|Default|SetGold (Math|Integer|Max(Integer) (+ Add (Variables|Default|GetGold)))))
  (return _output_get))

(fn AddCompletedLevel
  (params (MapName :type Name%20%28by%20ref%29))
  (Utilities|Array|AddUnique (Variables|Default|GetCompletedLevels) MapName))

(fn IsCompletedLevel
  (params (MapName :type Name%20%28by%20ref%29))
  (return (>= (Utilities|Array|FindItem (Variables|Default|GetCompletedLevels) MapName) 0)))