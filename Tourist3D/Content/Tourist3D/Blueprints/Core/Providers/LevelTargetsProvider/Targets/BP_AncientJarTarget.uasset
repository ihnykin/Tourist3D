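; BP_AncientJarTarget is an ancient jar level target that is collected when something overlaps it.
; On BeginPlay it binds to its StaticMesh's begin-overlap event, with no check on which actor overlaps.
; An overlap broadcasts OnTargetCollected with the jar and its TargetName, plays the Breaker sound at the game settings' sound volume, then destroys the actor.
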(event Custom|OnOverlapped_Event
  (params (OverlappedComponent :type Primitive%20Component%20Object%20Reference) (OtherActor :type Actor%20Object%20Reference) (OtherComp :type Primitive%20Component%20Object%20Reference) (OtherBodyIndex :type Integer) (bFromSweep :type Boolean) (SweepResult :type Hit%20Result%20Structure%20%28by%20ref%29))
  (Default|CallOnTargetCollected self (Variables|Default|GetTargetName))
  (Audio|PlaySoundatLocation "/Game/Tourist3D/Resources/Sound/Click/Breaker.Breaker" (Transformation|GetActorLocation) "0, 0, 0" (Variables|/Game/Tourist3D/Blueprints/Core/Providers/SaveGameProvider/BP_SaveGameProvider.BP_SaveGameProvider_C|GetGame%20Sounds%20Volume (CallFunction|GetMyGameSettings)) 1.0 0.0 0 0 0)
  (Actor|DestroyActor))

(event EventBeginPlay
  (Collision|BindEventtoOnComponentBeginOverlap (Variables|Default|GetStaticMesh) (delegate Custom|OnOverlapped_Event)))

(fn ConstructionScript)