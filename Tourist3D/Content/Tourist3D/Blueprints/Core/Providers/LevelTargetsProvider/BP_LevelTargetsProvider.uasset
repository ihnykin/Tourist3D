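; Level targets provider that tracks how many collection targets of each type exist in the level and how much is collected.
; On BeginPlay it runs a guarded one-time scan of all BP_BaseCollectionTarget actors, binding their collected events and counting totals per name enum in a map.
; Each pickup adds its weight to the collected count and rebroadcasts the updated counter.
; Getters expose names, counters and display info from DT_LevelTargetsInfo.
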(event Custom|OnCollectionTargetCollected_CustomEvent
  (params (TargetActor :type BP%20Base%20Collection%20Target%20Object%20Reference) (TargetName :type ETargetName%20Enum :default "NewEnumerator2") (TargetWeight :type Integer))
  (CollectionTargets|AddCollectionTargetPrivate TargetName TargetWeight)
  (bind (_name _counter) (CollectionTargets|GetCollectionTargetCounters TargetName))
  (Default|CallOnCollectionTargetCollected _name TargetWeight _counter))

(event EventBeginPlay
  (CallFunction|Initialize false))

(fn ConstructionScript)

(fn InitCollectionTargetsPrivate
  ;[1 1 1] [CollectionTargets]
  (bind _outactors (Actor|GetAllActorsOfClass "/Game/Tourist3D/Blueprints/Core/Providers/LevelTargetsProvider/CollectionTargets/BP_BaseCollectionTarget.BP_BaseCollectionTarget_C"))
  (for _array_element _outactors
    (EventDispatchers|BindEventtoOnTargetCollected _array_element (EventDispatchers|CreateEvent :!event Custom|OnCollectionTargetCollected_CustomEvent))
    (CollectionTargets|NewCollectionTargetTotalPrivate (Variables|/Game/Tourist3D/Blueprints/Core/Providers/LevelTargetsProvider/CollectionTargets/BP_BaseCollectionTarget.BP_BaseCollectionTarget_C|GetTargetName _array_element))))

(fn NewCollectionTargetTotalPrivate
  (params (TargetName :type ETargetName%20Enum :default "NewEnumerator2") (TargetWeight :type Integer))
  (bind _collectiontargetcounters (Variables|Default|GetCollectionTargetCounters))
  (bind (_value _returnvalue) (Utilities|Map|Find _collectiontargetcounters TargetName))
  (if _returnvalue
    (bind _structout (Utilities|Struct|SetmembersinFCollectionTargetCounter _value (+ (.TotalAmount (Utilities|Struct|BreakFCollectionTargetCounter _value)) 1)))
    (Utilities|Map|Add (Variables|Default|GetCollectionTargetCounters) TargetName _structout)
    (else
      (Utilities|Map|Add (Variables|Default|GetCollectionTargetCounters) TargetName (Utilities|Struct|MakeFCollectionTargetCounter 1)))))

(fn AddCollectionTargetPrivate
  (params (TargetName :type ETargetName%20Enum :default "NewEnumerator2") (TargetWeight :type Integer))
  (bind _collectiontargetcounters (Variables|Default|GetCollectionTargetCounters))
  (bind (_value _returnvalue) (Utilities|Map|Find _collectiontargetcounters TargetName))
  (if _returnvalue
    (bind _structout (Utilities|Struct|SetmembersinFCollectionTargetCounter _value (+ (.CollectedAmount (Utilities|Struct|BreakFCollectionTargetCounter _value)) TargetWeight)))
    (Utilities|Map|Add (Variables|Default|GetCollectionTargetCounters) TargetName _structout)))

(fn GetCollectionTargetNames
  (bind _keys (Utilities|Map|Keys (Variables|Default|GetCollectionTargetCounters)))
  (return _keys))

(fn GetCollectionTargetCounters
  (params (TargetName :type ETargetName%20Enum :default "NewEnumerator2"))
  (return TargetName (.Value (Utilities|Map|Find (Variables|Default|GetCollectionTargetCounters) TargetName))))

(fn PrintCollectionTargetCounters
  (if (Class|CommonUtils|IsDebugBuild)
    (bind _names (CollectionTargets|GetCollectionTargetNames))
    (for _array_element _names
      (Utilities|DebugInfo self (Utilities|String|EnumtoString _array_element) (Utilities|String|Append "Total = " (Utilities|String|ToString(Integer) (.totalamount (.Value (Utilities|Map|Find (Variables|Default|GetCollectionTargetCounters) _array_element)))) "; Collected = " (Utilities|String|ToString(Integer) (.collectedamount (.Value (Utilities|Map|Find (Variables|Default|GetCollectionTargetCounters) _array_element)))))))))

(fn Initialize
  (params (Force :type Boolean))
  (if (or Force (not (Variables|Default|GetIsInitialized)))
    (CollectionTargets|InitCollectionTargetsPrivate)
    (Variables|Default|SetIsInitialized true)))

(fn GetTargetInfo
  (params (TargetName :type ETargetName%20Enum :default "NewEnumerator2"))
  (bind _returnvalue (Utilities|GetDataTableRow "/Game/Tourist3D/Settings/DataTables/DT_LevelTargetsInfo.DT_LevelTargetsInfo" (Utilities|String|StringToName (Utilities|String|EnumtoString TargetName)))
    (:then
      (return _returnvalue))
    (:RowNotFound
      (return ""))))