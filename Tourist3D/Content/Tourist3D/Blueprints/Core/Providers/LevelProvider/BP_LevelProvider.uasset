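; BP_LevelProvider is the central access point for level data and level switching in the game.
; It looks up level info in the DT_LevelsInfo data table by map name, including for the currently loaded level.
; Its sorted list puts uncompleted levels first, then completed ones from the game settings stats, skipping IDs missing from the table.
; It also opens levels by map name and loads or detects the MapStartMenu start level.
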(fn ConstructionScript)

(fn GetSortedLevelList
  (bind _outrownames (DataTable|GetDataTableRowNames "/Game/Tourist3D/Settings/DataTables/DT_LevelsInfo.DT_LevelsInfo"))
  (for _array_element _outrownames
    ;[1 1 1] Not completed first
    (if (not (Default|IsCompletedLevel (CallFunction|GetMyGameSettings) _array_element))
      (Utilities|Array|Add (LocalVariables|GetLevelsLoc) _array_element)))
  ;[1 1 1] Reversed completed last
  (for _array_element_2 (.CompletedLevels (Default|GetStats (CallFunction|GetMyGameSettings)))
    (Utilities|GetDataTableRow "/Game/Tourist3D/Settings/DataTables/DT_LevelsInfo.DT_LevelsInfo" _array_element_2 ; TODO:: Sometimes id adds bad level
      (:then
        (Utilities|Array|Add (LocalVariables|GetLevelsLoc) _array_element_2))))
  (return (LocalVariables|GetLevelsLoc)))

(fn GetLevelInfo
  (params (MapName :type Name))
  (bind _returnvalue (Utilities|GetDataTableRow "/Game/Tourist3D/Settings/DataTables/DT_LevelsInfo.DT_LevelsInfo" MapName)
    (:then
      (return _returnvalue))))

(fn GetCurrentLevelInfo
  (bind _returnvalue (Game|GetCurrentLevelName true))
  (bind _levelinfo (CallFunction|GetLevelInfo (Utilities|String|StringToName _returnvalue)))
  (return _levelinfo))

(fn LoadLevel
  (params (LevelInfo :type F%20Level%20Info%20Structure%20%28by%20ref%29))
  (Game|OpenLevel(byName) (.mapname LevelInfo)))

(fn LoadStartLevel
  (Game|OpenLevel(byName) "MapStartMenu"))

(fn IsStartLevel
  (bind _returnvalue (Game|GetCurrentLevelName true))
  (return (Utilities|Enum|Equal(Enum) _returnvalue "MapStartMenu")))