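; BPL_Common is a function library that gives shortcut access to the game's MyGameInstance and the providers it holds.
; GetMyGameInstance casts the current game instance and logs a "Bad game instance" debug error if the cast fails.
; The other getters build on it to return the UI provider, the effect provider and, as game settings, the save game provider.
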(fn GetMyGameInstance
  (bind _asmy_game_instance (Utilities|Casting|CastToMyGameInstance (Game|GetGameInstance (LocalVariables|Get__WorldContext)))
    (:then
      _)
    (:CastFailed
      (Utilities|DebugError 0 "BPL_Common | " "Bad game instance"
        (:Out
          _))))
  (return _asmy_game_instance))

(fn GetMyUIProvider
  (return (Variables|/Game/Tourist3D/Blueprints/Core/MyGameInstance.MyGameInstance_C|GetUIProvider (CallFunction|GetMyGameInstance (LocalVariables|Get__WorldContext)))))

(fn GetMyEffectProvider
  (return (Variables|/Game/Tourist3D/Blueprints/Core/MyGameInstance.MyGameInstance_C|GetEffectProvider (CallFunction|GetMyGameInstance (LocalVariables|Get__WorldContext)))))

(fn GetMyGameSettings
  (return (Variables|/Game/Tourist3D/Blueprints/Core/MyGameInstance.MyGameInstance_C|GetSaveGameProvider (CallFunction|GetMyGameInstance (LocalVariables|Get__WorldContext)))))