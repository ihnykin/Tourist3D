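; Level gameplay Blueprint that runs the opening sequence when play begins on a map.
; After a short delay, it finds the map's BP_SpaceRocket, triggers RocketTakeoff and shows the space fade, logging an error if no rocket exists.
; It then opens the HUD through the UI provider unless the level provider reports the start level.
; Despite the PlayRocketLandingEffect name, the landing and hide-space calls are disconnected.
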(event Custom|StartPlayLevel
  (Utilities|FlowControl|Delay 0.2)
  (CallFunction|PlayRocketLandingEffect)
  ;[1 1 1] Add default UI
  (bind _isstartlevel (Default|IsStartLevel (CallFunction|GetMyLevelProvider)))
  (if (not _isstartlevel)
    (Default|OpenHUD (CallFunction|GetMyUIProvider))))

(event Custom|PlayRocketLandingEffect
  (bind _returnvalue (Actor|GetActorOfClass "/Game/Tourist3D/Blueprints/Characters/BP_SpaceRocket.BP_SpaceRocket_C"))
  (Utilities|IsValid _returnvalue
    (:Is%20Valid
      (Default|RocketTakeoff _returnvalue)
      (Default|ShowSpace (Default|GetSpaceFadeEffect (CallFunction|GetMyEffectProvider)) 3.5 false))
    (:Is%20Not%20Valid
      (Utilities|DebugError self "No space rocket on map found. Add BP_SpaceRocket on map."))))

(event EventBeginPlay
  (CallFunction|StartPlayLevel))

(fn ConstructionScript)