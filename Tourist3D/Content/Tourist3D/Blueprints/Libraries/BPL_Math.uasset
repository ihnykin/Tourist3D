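; Blueprint math function library for the Tourist3D project with small vector and sign helpers.
; VectorCos3D returns the cosine of the angle between two vectors from their dot product and lengths.
; IsPointUnderPlane uses it to compare the plane's up vector with the point-to-plane-origin direction, returning true when the cosine exceeds Delta.
; SetNNSign writes a float's sign into a by-ref variable, leaving it unchanged for zero.
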(fn VectorCos3D
  (params (NewParam :type Vector) (NewParam1 :type Vector))
  (return (/ (Math|Vector|DotProduct NewParam NewParam1) (* (Math|Vector|VectorLength NewParam) (Math|Vector|VectorLength NewParam1)))))

(fn IsPointUnderPlane
  (params (Plane :type Mesh%20Component%20Object%20Reference) (Point :type Vector) (Delta :type Float%20%28single-precision%29))
  (return (> (CallFunction|VectorCos3D (Math|Vector|GetUpVector Plane) (- (Transformation|GetWorldLocation Plane) Point) (LocalVariables|Get__WorldContext)) Delta)))

(fn SetNNSign
  (params (Value :type Float%20%28single-precision%29) (Ref :type Float%20%28single-precision%29%20%28by%20ref%29))
  (bind _returnvalue (Math|Float|Sign(Float) Value))
  (if (not (== _returnvalue 0.0))
    (|SetBy-RefVar Ref _returnvalue)))