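; Blueprint function library of common static helpers for the Tourist3D project.
; DebugError and DebugInfo print messages tagged with an object name, with errors in red.
; VectorCos3D returns the cosine between two vectors, which IsPointUnderPlane compares against a Delta threshold using the plane's up vector.
; GetMyEffectProvider fetches the EffectProvider from MyGameMode, reporting an error if the cast fails.
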(fn DebugError
  (params (Object :type Object%20Object%20Reference) (Msg1 :type String) (Msg2 :type String))
  (Development|PrintString 0 (Utilities|String|Append "ERROR | " (Utilities|GetObjectName Object) " | " Msg1 Msg2) true true "(R=1.000000,G=0.000000,B=0.000000,A=1.000000)" 5.0))

(fn DebugInfo
  (params (Object :type Object%20Object%20Reference) (Msg1 :type String) (Msg2 :type String))
  (Development|PrintString 0 (Utilities|String|Append "INFO | " (Utilities|GetObjectName Object) " | " Msg1 Msg2)))

(fn VectorCos3D
  (params (v1 :type Vector) (v2 :type Vector))
  (return (/ (Math|Vector|DotProduct v1 v2) (* (Math|Vector|VectorLength v1) (Math|Vector|VectorLength v2)))))

(fn IsPointUnderPlane
  (params (Plane :type Static%20Mesh%20Component%20Object%20Reference) (Point :type Vector) (Delta :type Float%20%28single-precision%29))
  (return (> (CallFunction|VectorCos3D (Math|Vector|GetUpVector Plane) (- (Transformation|GetWorldLocation Plane) Point) (LocalVariables|Get__WorldContext)) Delta)))

(fn GetMyEffectProvider
  (bind _asmy_game_mode (Utilities|Casting|CastToMyGameMode (Game|GetGameMode (LocalVariables|Get__WorldContext)))
    (:then
      _)
    (:CastFailed
      (CallFunction|DebugError 0 "BPL_Common | " "Invalid effect provider" (LocalVariables|Get__WorldContext))))
  (return (Variables|/Game/Tourist3D/Blueprints/MyGameMode.MyGameMode_C|GetEffectProvider _asmy_game_mode)))