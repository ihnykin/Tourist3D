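; BP_LevelProvider supplies level lists and level info and handles switching between levels and the start menu.
; The sorted list takes row names from DT_LevelsInfo, putting uncompleted levels first, then appending the completed levels saved in game settings.
; Level info comes from the matching table row and is filled in through game settings.
; Loading opens maps by name, and a name check identifies the MapStartMenu level.
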(fn ConstructionScript)

(fn GetSortedLevelList
  (bind _outrownames (DataTable|GetDataTableRowNames "/Game/Tourist3D/Maps/DT_LevelsInfo.DT_LevelsInfo"))
  (for _array_element _outrownames
    ;[1 1 1] Not completed first
    (if (not (>= (Utilities|Array|FindItem (Variables|/Game/Tourist3D/Blueprints/Core/SaveGameProvider/BP_SaveGameProvider.BP_SaveGameProvider_C|GetCompletedLevels (CallFunction|GetMyGameSettings)) _array_element) 0))
      (Utilities|Array|Add (LocalVariables|GetLevelsLoc) _array_element)))
  ;[1 1 1] Reversed completed last
  (for _array_element_2 (Variables|/Game/Tourist3D/Blueprints/Core/SaveGameProvider/BP_SaveGameProvider.BP_SaveGameProvider_C|GetCompletedLevels (CallFunction|GetMyGameSettings))
    (Utilities|Array|Add (LocalVariables|GetLevelsLoc) _array_element_2))
  (return (LocalVariables|GetLevelsLoc)))

(fn GetLevelInfo
  (params (MapName :type Name))
  (bind _returnvalue (Utilities|GetDataTableRow "/Game/Tourist3D/Maps/DT_LevelsInfo.DT_LevelsInfo" MapName)
    (:then
      ;[1 1 1] Fill Level Info Step2
      (bind _levelinfoex (Default|FillLevelInfo (CallFunction|GetMyGameSettings) (Utilities|Struct|MakeFLevelInfoEx _returnvalue false)))
      (return _levelinfoex))))

(fn LoadLevel
  (params (LevelInfo :type F%20Level%20Info%20Structure%20%28by%20ref%29))
  (Game|OpenLevel(byName) (.mapname LevelInfo)))

(fn LoadStartLevel
  (Game|OpenLevel(byName) "MapStartMenu"))

(fn IsStartLevel
  (bind _returnvalue (Game|GetCurrentLevelName true))
  (return (Utilities|Enum|Equal(Enum) _returnvalue "MapStartMenu")))